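; BP_Monster is a monster that attaches to the player's attach point and attacks by rotating its body.
; Each tick plays the Retract timeline while the player looks and stands in front of a mirror, otherwise Rotate.
; Chained timelines drive body roll: Retract restarts Rotate, which leads into QuickRotate.
; When QuickRotate finishes, it damages the player, launches them with random horizontal velocity and retracts.
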(event EventBeginPlay
  (bind _asl1_character (Utilities|Casting|CastToL1_Character (Game|GetPlayerCharacter 0)))
  (bind _output_get (Variables|Default|SetPlayerRef _asl1_character))
  (Transformation|AttachComponentToComponent (Variables|Default|GetDefaultSceneRoot) (Variables|/Game/Blueprints/Game/Level1/L1_Character.L1_Character_C|GetAttachPoint _output_get) "None" "SnapToTarget" "KeepRelative" "KeepRelative" true))

(event EventTick
  (params (DeltaSeconds :type Float%20%28single-precision%29))
  (bind _playerref (Variables|Default|GetPlayerRef))
  (bind _playerref_2 (Variables|Default|GetPlayerRef))
  (if (and (Variables|/Game/Blueprints/Game/Level1/L1_Character.L1_Character_C|GetIsLooking? _playerref_2) (Variables|/Game/Blueprints/Game/Level1/L1_Character.L1_Character_C|GetIsInFrontOfMirror? _playerref_2))
    (bind _newtrack_0 (Timeline|Retract Play)
      (:Update
        (Transformation|SetRelativeRotation (Variables|Default|GetBody) (Math|Rotator|MakeRotator _newtrack_0 0.0 0.0) false false))
      (:Finished
        (bind _newtrack_0_2 (Timeline|Rotate PlayFromStart)
          (:Update
            (Transformation|SetRelativeRotation (Variables|Default|GetBody) (Math|Rotator|MakeRotator _newtrack_0_2 0.0 0.0) false false))
          (:Finished
            (bind _newtrack_0_3 (Timeline|QuickRotate Play)
              (:Update
                (Transformation|SetRelativeRotation (Variables|Default|GetBody) (Math|Rotator|MakeRotator _newtrack_0_3 0.0 0.0) false false))
              (:Finished
                (Game|Damage|ApplyDamage _playerref 25.0 0 0)
                (Character|LaunchCharacter _playerref (Math|Vector|MakeVector (* (Math|Random|RandomFloat) 1e+04) (* (Math|Random|RandomFloat) 1e+04) 0.0) false false)
                (Timeline|Retract Play)))))))
    (else
      (Timeline|Rotate Play))))

(fn ConstructionScript)