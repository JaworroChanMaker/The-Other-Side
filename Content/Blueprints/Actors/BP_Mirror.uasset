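; BP_Mirror is a mirror actor that tells the L1_Character player when it is in front of the glass and how far away it is.
; Box overlap events toggle the player's IsInFrontOfMirror flag without checking which actor overlaps, and clear IsLooking on exit.
; While flagged, Tick runs RayCastMirror, tracing the Camera channel from Glass to the player's camera.
; It writes the hit distance and the sum of both locations to the character.
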(event OnComponentBeginOverlap(Box)
  (params (OverlappedComponent :type Primitive%20Component%20Object%20Reference) (OtherActor :type Actor%20Object%20Reference) (OtherComp :type Primitive%20Component%20Object%20Reference) (OtherBodyIndex :type Integer) (bFromSweep :type Boolean) (SweepResult :type Hit%20Result%20Structure%20%28by%20ref%29))
  (bind _asl1_character (Utilities|Casting|CastToL1_Character (Variables|Default|GetPlayerRef)))
  (Variables|/Game/Blueprints/Game/Level1/L1_Character.L1_Character_C|SetIsInFrontOfMirror? _asl1_character true)
  (CallFunction|RayCastMirror))

(event OnComponentEndOverlap(Box)
  (params (OverlappedComponent :type Primitive%20Component%20Object%20Reference) (OtherActor :type Actor%20Object%20Reference) (OtherComp :type Primitive%20Component%20Object%20Reference) (OtherBodyIndex :type Integer))
  (bind _asl1_character (Utilities|Casting|CastToL1_Character (Variables|Default|GetPlayerRef)))
  (Variables|/Game/Blueprints/Game/Level1/L1_Character.L1_Character_C|SetIsInFrontOfMirror? _asl1_character false)
  (Variables|Default|SetIsLooking? false))

(event EventTick
  (params (DeltaSeconds :type Float%20%28single-precision%29))
  (if (Variables|/Game/Blueprints/Game/Level1/L1_Character.L1_Character_C|GetIsInFrontOfMirror? (Variables|Default|GetPlayerRef))
    (CallFunction|RayCastMirror)))

(event EventBeginPlay
  (bind _asl1_character (Utilities|Casting|CastToL1_Character (Game|GetPlayerCharacter 0)))
  (Variables|Default|SetPlayerRef _asl1_character))

(fn ConstructionScript)

(fn RayCastMirror
  (bind _glass (Variables|Default|GetGlass))
  (bind _returnvalue (Transformation|GetWorldLocation _glass))
  (bind _asl1_character (Utilities|Casting|CastToL1_Character (Game|GetPlayerCharacter 0)))
  (Variables|/Game/Blueprints/Game/Level1/L1_Character.L1_Character_C|SetMirrorCastVector _asl1_character (+ _returnvalue (Transformation|GetWorldLocation (Variables|/Game/Blueprints/Game/Level1/L1_Character.L1_Character_C|GetCamera _asl1_character))))
  (bind _outhit (Collision|LineTraceByChannel _returnvalue (Transformation|GetWorldLocation (Variables|/Game/Blueprints/Game/Level1/L1_Character.L1_Character_C|GetCamera _asl1_character)) "TraceTypeQuery2" false 0 "None"))
  (Variables|/Game/Blueprints/Game/Level1/L1_Character.L1_Character_C|SetDistanceFromMirror (Variables|Default|GetPlayerRef) (.distance _outhit)))